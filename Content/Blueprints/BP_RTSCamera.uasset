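; RTS camera pawn for commanding ships, with panning, spring-arm zoom, hold-to-rotate and two HUD widgets for entity details and reinforcements.
; Select traces under the cursor to pick ships or hardpoints, highlighting via custom depth with a timer-positioned details panel; release places reinforcement holograms.
; Alt-Select cancels active reinforcements, assigns turret targets and spawns movement markers where the cursor ray meets a horizontal plane, raised by ship-class Z level.
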(event EventBeginPlay
  (bind _returnvalue (Game|GetPlayerController 0))
  (bind _returnvalue_2 (Game|GetPlayerController 0))
  (bind _player_colour (Variables|Default|GetPlayer%20Colour))
  ;[1 1 1] Begin Play Events
  (Utilities|FlowControl|Sequence
    (:then_0
      (bind _returnvalue_3 (Settings|GetGameUserSettings))
      (Class|GameUserSettings|SetFullscreenMode _returnvalue_3 "WindowedFullscreen")
      (Input|SetInputModeGameandUI _returnvalue 0 "DoNotLock" false)
      (Variables|/Script/Engine.PlayerController|SetbShowMouseCursor _returnvalue true))
    (:then_1
      (bind _returnvalue_4 (UserInterface|CreateWidget "/Game/Blueprints/HUD_EntityDetails.HUD_EntityDetails_C" _returnvalue_2 _player_colour))
      (Variables|Default|SetSelected%20Entity%20HUD _returnvalue_4))
    (:then_2
      (bind _returnvalue_5 (UserInterface|CreateWidget "/Game/Blueprints/HUD_ReinforcementPanel.HUD_ReinforcementPanel_C" _returnvalue_2 _player_colour self))
      (bind _output_get (Variables|Default|SetHUD%20Reinforcement%20Panel%20Ref _returnvalue_5))
      (UserInterface|Viewport|AddtoViewport _output_get 0))))

(event Input|ActionEvents|InputActionSelect
  (params (Key :type Key%20Structure :default "None"))
  ;[1 1 1] Selection
  (:Pressed
    ;;[1 1 1] Should be final check
    (CallFunction|EntitySelection))
  (:Released
    (CallFunction|ReinforcementPlacement)))

(event Input|ActionEvents|InputActionAlt-Select
  (params (Key :type Key%20Structure :default "None"))
  ;[1 1 1] Alternative Selection
  (:Pressed
    (CallFunction|DeselectReinforcement)
    (CallFunction|TargetingforSelection)
    (CallFunction|SetShipMovementTarget)))

(event Input|ActionEvents|InputActionRotateCamera
  (params (Key :type Key%20Structure :default "None"))
  (bind _sphere (Variables|Default|GetSphere))
  (bind _returnvalue (Transformation|GetWorldRotation _sphere))
  ;[1 1 1] Rotate
  (:Pressed
    (Utilities|FlowControl|Gate true) ; enters at Open
  )
  (:Released
    (Transformation|SetWorldRotation _sphere "-45.000000, 0,0.000000" false false)
    (Utilities|FlowControl|Gate true) ; enters at Close
  ))

(event Input|AxisEvents|InputAxisCameraForward/Back
  (params (AxisValue :type Float%20%28single-precision%29))
  ;[1 1 1] Movement
  (Class|PawnMovementComponent|AddInputVector (Variables|Default|GetFloatingPawnMovement) (Math|Vector|RotateVector (Math|Vector|MakeVector AxisValue (stale Input|AxisEvents|InputAxisCameraLeft/Right AxisValue) 0.0) (Math|Rotator|MakeRotator 0.0 0.0 (.yaw (Transformation|GetWorldRotation (Variables|Default|GetSphere))))) false))

(event Input|AxisEvents|InputAxisCameraLeft/Right
  (params (AxisValue :type Float%20%28single-precision%29))
  ;[1 1 1] Movement
  (Class|PawnMovementComponent|AddInputVector (Variables|Default|GetFloatingPawnMovement) (Math|Vector|RotateVector (Math|Vector|MakeVector (stale Input|AxisEvents|InputAxisCameraForward/Back AxisValue) AxisValue 0.0) (Math|Rotator|MakeRotator 0.0 0.0 (.yaw (Transformation|GetWorldRotation (Variables|Default|GetSphere))))) false))

(event Input|AxisEvents|InputAxisCameraZoom
  (params (AxisValue :type Float%20%28single-precision%29))
  (bind _springarm (Variables|Default|GetSpringArm))
  ;[1 1 1] Zoom
  (Variables|/Script/Engine.SpringArmComponent|SetTargetArmLength _springarm (Math|Float|Clamp(Float) (+ (Variables|/Script/Engine.SpringArmComponent|GetTargetArmLength _springarm) (* AxisValue 1e+02)) 7e+02 7e+03)))

(event Input|MouseEvents|MouseX
  (params (AxisValue :type Float%20%28single-precision%29))
  (bind _sphere (Variables|Default|GetSphere))
  (bind _returnvalue (Transformation|GetWorldRotation _sphere))
  ;[1 1 1] Rotate
  (Utilities|FlowControl|Gate true
    (:Exit
      (Transformation|SetWorldRotation _sphere (Math|Rotator|MakeRotator 0.0 (Math|Float|ClampAngle (+ (stale Input|MouseEvents|MouseY AxisValue) (.pitch _returnvalue)) -89.0 89.0) (+ (.yaw _returnvalue) AxisValue)) false false))))

(event Input|MouseEvents|MouseY
  (params (AxisValue :type Float%20%28single-precision%29))
  (bind _sphere (Variables|Default|GetSphere))
  (bind _returnvalue (Transformation|GetWorldRotation _sphere))
  ;[1 1 1] Rotate
  (Utilities|FlowControl|Gate true
    (:Exit
      (Transformation|SetWorldRotation _sphere (Math|Rotator|MakeRotator 0.0 (Math|Float|ClampAngle (+ AxisValue (.pitch _returnvalue)) -89.0 89.0) (+ (.yaw _returnvalue) (stale Input|MouseEvents|MouseX AxisValue))) false false))))

(fn ConstructionScript)

(fn PositionSelectedUnitHUD
  (Class|UserWidget|SetPositioninViewport (Variables|Default|GetSelected%20Entity%20HUD) (.ScreenPosition (Class|GameplayStatics|ProjectWorldtoScreen (Game|GetPlayerController 0) (Transformation|GetActorLocation (Variables|Default|GetSelected%20Entity)) true)) true))

(fn EntitySelection
  (Utilities|IsValid (Variables|Default|GetSelected%20Entity)
    (:Is%20Valid
      ;[1 1 1] Hide Ship Stuff
      (bind _asship_master (Utilities|Casting|CastToShip_Master (Variables|Default|GetSelected%20Entity))
        (:then
          (for _array_element (Variables|/Game/Entities/Ship_Master.Ship_Master_C|GetActive%20Hardpoints _asship_master)
            (Rendering|SetVisibility (Variables|/Game/Entities/Hardpoint_Master.Hardpoint_Master_C|GetHUD%20Icon _array_element) false false))
          (Utilities|IsValid (Variables|/Game/Entities/Ship_Master.Ship_Master_C|GetMovement%20Marker _asship_master)
            (:Is%20Valid
              (Actor|DestroyActor (Variables|/Game/Entities/Ship_Master.Ship_Master_C|GetMovement%20Marker _asship_master))
              (Variables|/Game/Entities/Ship_Master.Ship_Master_C|SetMovement%20Marker _asship_master 0))
            (:Is%20Not%20Valid
              _)))
        (:CastFailed
          _))
      (Utilities|FormatSelectionDetails true
        (:exec%20out
          _)))
    (:Is%20Not%20Valid
      _))
  ;[1 1 1] Get Target
  (bind _outhit (Collision|LineTraceByChannel (Transformation|GetWorldLocation (Variables|Default|GetCamera)) (.Location (Collision|BreakHitResult (.HitResult (Game|Player|GetHitResultUnderCursorbyChannel (Game|GetPlayerController 0) "TraceTypeQuery1" true)))) "TraceTypeQuery2" true 0 "None"))
  ;[1 1 1] Set Target
  (if (Math|Vector|NotEqual(Vector) (.traceend _outhit) "0, 0, 0" 0.0001)
    (bind _asship_master_2 (Utilities|Casting|CastToShip_Master (.hitactor _outhit))
      (:then
        (Variables|Default|SetSelected%20Entity _asship_master_2)
        (Utilities|FormatSelectionDetails false
          (:exec%20out
            (for _array_element_2 (Variables|/Game/Entities/Ship_Master.Ship_Master_C|GetActive%20Hardpoints _asship_master_2)
              (Rendering|SetVisibility (Variables|/Game/Entities/Hardpoint_Master.Hardpoint_Master_C|GetHUD%20Icon _array_element_2) true false)))))
      (:CastFailed
        (bind _ashardpoint_master (Utilities|Casting|CastToHardpoint_Master (.hitactor _outhit)))
        (Variables|Default|SetSelected%20Entity _ashardpoint_master)
        (Utilities|FormatSelectionDetails false)))))

(fn ReinforcementPlacement
  (bind _hud_reinforcement_panel_ref (Variables|Default|GetHUD%20Reinforcement%20Panel%20Ref))
  (bind _current_hologram (Variables|/Game/Blueprints/HUD_ReinforcementPanel.HUD_ReinforcementPanel_C|GetCurrent%20Hologram _hud_reinforcement_panel_ref))
  (Utilities|IsValid _current_hologram
    (:Is%20Valid
      (Default|BeginJump _current_hologram)
      (Default|SetCurrentActive _hud_reinforcement_panel_ref 0 false))
    (:Is%20Not%20Valid
      (return))))

(fn TargetingforSelection
  (bind _selected_entity (Variables|Default|GetSelected%20Entity))
  (Utilities|IsValid (Variables|Default|GetSelected%20Entity)
    (:Is%20Valid
      (bind _outhit (Collision|LineTraceByChannel (Transformation|GetWorldLocation (Variables|Default|GetCamera)) (.Location (Collision|BreakHitResult (.HitResult (Game|Player|GetHitResultUnderCursorbyChannel (Game|GetPlayerController 0) "TraceTypeQuery1" true)))) "TraceTypeQuery2" true 0 "None"))
      (if (Math|Vector|NotEqual(Vector) (.traceend _outhit) "0, 0, 0" 0.0001)
        (bind _asship_master (Utilities|Casting|CastToShip_Master (.hitactor _outhit))
          (:then
            (LocalVariables|SetNew%20Target _asship_master))
          (:CastFailed
            (bind _ashardpoint_master (Utilities|Casting|CastToHardpoint_Master (.hitactor _outhit))
              (:then
                (LocalVariables|SetNew%20Target _ashardpoint_master))
              (:CastFailed
                (return)))))
        (bind _asship_master_2 (Utilities|Casting|CastToShip_Master _selected_entity)
          (:then
            (Default|SetTurretsTarget _asship_master_2 (LocalVariables|GetNew%20Target)))
          (:CastFailed
            (bind _asturret_master (Utilities|Casting|CastToTurret_Master _selected_entity))
            (Variables|/Game/Entities/Turret_Master.Turret_Master_C|SetTarget%20Entity _asturret_master (LocalVariables|GetNew%20Target))))))
    (:Is%20Not%20Valid
      (return))))

(fn DeselectReinforcement
  (bind _hud_reinforcement_panel_ref (Variables|Default|GetHUD%20Reinforcement%20Panel%20Ref))
  (bind _current_active (Variables|/Game/Blueprints/HUD_ReinforcementPanel.HUD_ReinforcementPanel_C|GetCurrent%20Active _hud_reinforcement_panel_ref))
  (Utilities|IsValid _current_active
    (:Is%20Valid
      (Math|Integer|IncrementInt (Variables|/Game/Blueprints/HUD_ReinforcementIcon.HUD_ReinforcementIcon_C|GetNumber _current_active)
        (:%20%20
          (Default|SetCurrentActive _hud_reinforcement_panel_ref 0 true))))
    (:Is%20Not%20Valid
      (return))))

(fn SetShipMovementTarget
  (bind _returnvalue (Game|GetPlayerController 0))
  (bind _plane (Utilities|Struct|MakePlane 0.0 0.0 0.0 1.0))
  (bind _selected_entity (Variables|Default|GetSelected%20Entity))
  (bind (_worldlocation _worlddirection) (Game|Player|ConvertMouseLocationToWorldSpace _returnvalue))
  (bind _returnvalue_2 (* _worlddirection 9999999.0))
  (bind _returnvalue_3 (+ _worldlocation _returnvalue_2))
  (bind (_t _intersection _returnvalue_4) (Class|KismetMathLibrary|LinePlaneIntersection _worldlocation _returnvalue_3 _plane))
  (bind (_x _y _z) (Math|Vector|BreakVector _intersection))
  (Utilities|IsValid _selected_entity
    (:Is%20Valid
      (bind _asship_master (Utilities|Casting|CastToShip_Master _selected_entity))
      (if _returnvalue_4
        (bind _returnvalue_5 (Game|SpawnActorfromClass "/Game/Entities/ShipMovementMarker.ShipMovementMarker_C" (Math|Transform|MakeTransform (Math|Vector|MakeVector _x _y (+ _z (.Value (Utilities|Map|Find (.Ship%20Z%20Level (Utilities|GetClassDefaults (Utilities|GetClass _asship_master))) (.class (Variables|/Game/Entities/Ship_Master.Ship_Master_C|GetShip%20Details _asship_master)))))) "0, 0, 0" "0.100000,0.100000,0.100000") "Undefined" 0 0))
        (Default|SetNewMovementMarker _asship_master _returnvalue_5)))))