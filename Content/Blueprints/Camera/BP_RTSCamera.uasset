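; RTS camera pawn that handles view control, entity selection and reinforcement placement, and creates both related HUD widgets.
; Input pans relative to the Sphere's yaw, zooms the spring arm, and rotates through a gate while held, resetting on release.
; Clicks trigger any pending hologram's jump, then trace for ships or hardpoints.
; Selections get a custom-depth highlight and a details widget that a looping timer keeps at their screen position.
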(event EventBeginPlay
  (bind _returnvalue (Game|GetPlayerController 0))
  (bind _returnvalue_2 (Game|GetPlayerController 0))
  ;[1 1 1] Begin Play Events
  (Utilities|FlowControl|Sequence
    (:then_0
      (bind _returnvalue_3 (Settings|GetGameUserSettings))
      (Class|GameUserSettings|SetFullscreenMode _returnvalue_3 "WindowedFullscreen")
      (Input|SetInputModeGameandUI _returnvalue 0 "DoNotLock" false)
      (Variables|/Script/Engine.PlayerController|SetbShowMouseCursor _returnvalue true))
    (:then_1
      (bind _returnvalue_4 (UserInterface|CreateWidget "/Game/Blueprints/HUD/HUD_EntityDetails.HUD_EntityDetails_C" _returnvalue_2))
      (bind _output_get (Variables|Default|SetSelected%20Entity%20HUD _returnvalue_4))
      (Variables|/Game/Blueprints/HUD/HUD_EntityDetails.HUD_EntityDetails_C|SetPlayer%20Colour _output_get (Variables|Default|GetPlayer%20Colour)))
    (:then_2
      (bind _returnvalue_5 (UserInterface|CreateWidget "/Game/Blueprints/HUD/HUD_ReinforcementPanel.HUD_ReinforcementPanel_C" _returnvalue_2))
      (bind _output_get_2 (Variables|Default|SetHUD%20Reinforcement%20Panel%20Ref _returnvalue_5))
      (UserInterface|Viewport|AddtoViewport _output_get_2 0)
      (Variables|/Game/Blueprints/HUD/HUD_ReinforcementPanel.HUD_ReinforcementPanel_C|SetPlayerColour _returnvalue_5 (Variables|Default|GetPlayer%20Colour)))))

(event Input|ActionEvents|InputActionSelect
  (params (Key :type Key%20Structure :default "None"))
  ;[1 1 1] Selection
  (:Pressed
    (CallFunction|ReinforcementPlacement)
    ;;[1 1 1] Should be final check
    (CallFunction|EntitySelection)))

(event Input|ActionEvents|InputActionAlt-Select
  (params (Key :type Key%20Structure :default "None"))
  ;[1 1 1] Alternative Selection
  (:Pressed
    (Utilities|IsValid (Variables|/Game/Blueprints/HUD/HUD_ReinforcementPanel.HUD_ReinforcementPanel_C|GetCurrent%20Active (Variables|Default|GetHUD%20Reinforcement%20Panel%20Ref))
      (:Is%20Valid
        (Default|SetCurrentActive (Variables|Default|GetHUD%20Reinforcement%20Panel%20Ref))))))

(event Input|ActionEvents|InputActionRotateCamera
  (params (Key :type Key%20Structure :default "None"))
  (bind _sphere (Variables|Default|GetSphere))
  (bind _returnvalue (Transformation|GetWorldRotation _sphere))
  ;[1 1 1] Rotate
  (:Pressed
    (Utilities|FlowControl|Gate true) ; enters at Open
  )
  (:Released
    (Transformation|SetWorldRotation _sphere "-45.000000, 0,0.000000" false false)
    (Utilities|FlowControl|Gate true) ; enters at Close
  ))

(event Input|AxisEvents|InputAxisCameraForward/Back
  (params (AxisValue :type Float%20%28single-precision%29))
  ;[1 1 1] Movement
  (Class|PawnMovementComponent|AddInputVector (Variables|Default|GetFloatingPawnMovement) (Math|Vector|RotateVector (Math|Vector|MakeVector AxisValue (stale Input|AxisEvents|InputAxisCameraLeft/Right AxisValue) 0.0) (Math|Rotator|MakeRotator 0.0 0.0 (.yaw (Transformation|GetWorldRotation (Variables|Default|GetSphere))))) false))

(event Input|AxisEvents|InputAxisCameraLeft/Right
  (params (AxisValue :type Float%20%28single-precision%29))
  ;[1 1 1] Movement
  (Class|PawnMovementComponent|AddInputVector (Variables|Default|GetFloatingPawnMovement) (Math|Vector|RotateVector (Math|Vector|MakeVector (stale Input|AxisEvents|InputAxisCameraForward/Back AxisValue) AxisValue 0.0) (Math|Rotator|MakeRotator 0.0 0.0 (.yaw (Transformation|GetWorldRotation (Variables|Default|GetSphere))))) false))

(event Input|AxisEvents|InputAxisCameraZoom
  (params (AxisValue :type Float%20%28single-precision%29))
  (bind _springarm (Variables|Default|GetSpringArm))
  ;[1 1 1] Zoom
  (Variables|/Script/Engine.SpringArmComponent|SetTargetArmLength _springarm (Math|Float|Clamp(Float) (+ (Variables|/Script/Engine.SpringArmComponent|GetTargetArmLength _springarm) (* AxisValue 1e+02)) 2e+03 7e+03)))

(event Input|MouseEvents|MouseX
  (params (AxisValue :type Float%20%28single-precision%29))
  (bind _sphere (Variables|Default|GetSphere))
  (bind _returnvalue (Transformation|GetWorldRotation _sphere))
  ;[1 1 1] Rotate
  (Utilities|FlowControl|Gate true
    (:Exit
      (Transformation|SetWorldRotation _sphere (Math|Rotator|MakeRotator 0.0 (Math|Float|ClampAngle (+ (stale Input|MouseEvents|MouseY AxisValue) (.pitch _returnvalue)) -89.0 89.0) (+ (.yaw _returnvalue) AxisValue)) false false))))

(event Input|MouseEvents|MouseY
  (params (AxisValue :type Float%20%28single-precision%29))
  (bind _sphere (Variables|Default|GetSphere))
  (bind _returnvalue (Transformation|GetWorldRotation _sphere))
  ;[1 1 1] Rotate
  (Utilities|FlowControl|Gate true
    (:Exit
      (Transformation|SetWorldRotation _sphere (Math|Rotator|MakeRotator 0.0 (Math|Float|ClampAngle (+ AxisValue (.pitch _returnvalue)) -89.0 89.0) (+ (.yaw _returnvalue) (stale Input|MouseEvents|MouseX AxisValue))) false false))))

(fn ConstructionScript)

(fn PositionSelectedUnitHUD
  (Class|UserWidget|SetPositioninViewport (Variables|Default|GetSelected%20Entity%20HUD) (.ScreenPosition (Class|GameplayStatics|ProjectWorldtoScreen (Game|GetPlayerController 0) (Transformation|GetActorLocation (Variables|Default|GetSelected%20Entity)) true)) true))

(fn EntitySelection
  (Utilities|IsValid (Variables|Default|GetSelected%20Entity)
    (:Is%20Valid
      (Utilities|FormatSelectionDetails true
        (:exec%20out
          _)))
    (:Is%20Not%20Valid
      _))
  (bind _outhit (Collision|LineTraceByChannel (Transformation|GetWorldLocation (Variables|Default|GetCamera)) (.Location (Collision|BreakHitResult (.HitResult (Game|Player|GetHitResultUnderCursorbyChannel (Game|GetPlayerController 0) "TraceTypeQuery1" true)))) "TraceTypeQuery1" false 0 "ForDuration"))
  (if (Math|Vector|NotEqual(Vector) (.traceend _outhit) "0, 0, 0" 0.0001)
    (bind _asship_master (Utilities|Casting|CastToShip_Master (.hitactor _outhit))
      (:then
        (Variables|Default|SetSelected%20Entity _asship_master)
        (Utilities|FormatSelectionDetails false))
      (:CastFailed
        (bind _ashardpoint_master (Utilities|Casting|CastToHardpoint_Master (.hitactor _outhit)))
        (Variables|Default|SetSelected%20Entity _ashardpoint_master)
        (Utilities|FormatSelectionDetails false)))))

(fn ReinforcementPlacement
  (bind _hud_reinforcement_panel_ref (Variables|Default|GetHUD%20Reinforcement%20Panel%20Ref))
  (bind _current_hologram (Variables|/Game/Blueprints/HUD/HUD_ReinforcementPanel.HUD_ReinforcementPanel_C|GetCurrent%20Hologram _hud_reinforcement_panel_ref))
  (Utilities|IsValid _current_hologram
    (:Is%20Valid
      (Default|BeginJump _current_hologram)
      (Variables|/Game/Blueprints/HUD/HUD_ReinforcementPanel.HUD_ReinforcementPanel_C|SetCurrent%20Active _hud_reinforcement_panel_ref 0))
    (:Is%20Not%20Valid
      (return))))