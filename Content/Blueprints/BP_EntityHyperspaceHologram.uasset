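; Hologram placement preview for hyperspacing a reinforcement ship into the game, using the ship's mesh with a dynamic holo material.
; While tracking, it follows the cursor's ground-plane projection at the ship class's Z level.
; Simple overlap events mark it blocked and toggle the material.
; BeginJump deselects the reinforcement if blocked; otherwise it spawns the ship far behind, timeline-slides it in without collision, calls post-jump, then destroys itself.
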(event OnComponentBeginOverlap(StaticMesh)
  (params (OverlappedComponent :type Primitive%20Component%20Object%20Reference) (OtherActor :type Actor%20Object%20Reference) (OtherComp :type Primitive%20Component%20Object%20Reference) (OtherBodyIndex :type Integer) (bFromSweep :type Boolean) (SweepResult :type Hit%20Result%20Structure%20%28by%20ref%29))
  ;[1 1 1] Basic really really really bad overlap detection
  (Variables|Default|SetSafe%20To%20Jump? false)
  (Rendering|Material|SetScalarParameterValue (Variables|Default|GetDynMatIns) "Blocked" 1.0 :!class /Script/Engine.MaterialInstanceDynamic))

(event OnComponentEndOverlap(StaticMesh)
  (params (OverlappedComponent :type Primitive%20Component%20Object%20Reference) (OtherActor :type Actor%20Object%20Reference) (OtherComp :type Primitive%20Component%20Object%20Reference) (OtherBodyIndex :type Integer))
  ;[1 1 1] Basic really really really bad overlap detection
  (Variables|Default|SetSafe%20To%20Jump? true)
  (Rendering|Material|SetScalarParameterValue (Variables|Default|GetDynMatIns) "Blocked" 0.0 :!class /Script/Engine.MaterialInstanceDynamic))

(event Custom|Begin%20Jump
  (if (Variables|Default|GetSafe%20To%20Jump?)
    ;[1 1 1] Create Holo Mesh
    (Variables|Default|SetTracking%20Cursor? false)
    (Rendering|SetVisibility (Variables|Default|GetStaticMesh) false false)
    (bind _returnvalue (Game|SpawnActorfromClass (Variables|Default|GetEntity) (Math|Transform|MakeTransform (+ (Transformation|GetActorLocation) (* (Transformation|GetActorForwardVector) -1e+05)) (Transformation|GetActorRotation) "1.000000,1,1") "Undefined" 0 (Variables|Default|GetPlayer%20Pawn) 0))
    (bind _output_get (Variables|Default|SetActor _returnvalue))
    (bind _asship_master (Utilities|Casting|CastToShip_Master _output_get))
    (Rendering|SetActorHiddenInGame _asship_master true)
    (Utilities|FlowControl|Delay 1.0)
    (Rendering|SetActorHiddenInGame _asship_master false)
    (Collision|SetCollisionEnabled (Variables|/Game/Entities/Ship_Master.Ship_Master_C|GetPrimary%20Mesh _asship_master) "NoCollision")
    ;[1 1 1] Hyperspace Jump Animation
    (bind _x_pos_movement (Timeline|Hyperspace%20Jump PlayFromStart)
      (:Update
        (Transformation|SetActorLocation (Variables|Default|GetActor) (+ (* (Transformation|GetActorForwardVector) (* _x_pos_movement -1.0)) (Transformation|GetActorLocation)) false false))
      (:Finished
        (Collision|SetCollisionEnabled (Variables|/Game/Entities/Ship_Master.Ship_Master_C|GetPrimary%20Mesh _asship_master) "QueryAndPhysics")
        (Default|EventPostJump _asship_master)
        (Actor|DestroyActor)))
    (else
      (Default|DeselectReinforcement (Variables|Default|GetPlayer%20Pawn)))))

(event EventBeginPlay
  ;[1 1 1] Set Holo Material
  (bind _returnvalue (Rendering|Material|CreateDynamicMaterialInstance "/Game/Blueprints/Mat_HyperspaceHologram.Mat_HyperspaceHologram" (Utilities|String|StringToName (Utilities|GetObjectName self)) :!class /Script/Engine.KismetMaterialLibrary))
  (Variables|Default|SetDynMatIns _returnvalue))

(event EventTick
  (params (DeltaSeconds :type Float%20%28single-precision%29))
  (bind _returnvalue (Game|GetPlayerController 0))
  (bind _entity (Variables|Default|GetEntity))
  (bind (_worldlocation _worlddirection) (Game|Player|ConvertMouseLocationToWorldSpace _returnvalue))
  (bind (_ship_details _ship_stats _hardpoints _active_hardpoints _primary_static_mesh _ship_z_level) (Utilities|GetClassDefaults _entity))
  (bind _z (Math|Vector|BreakVector _worlddirection))
  (bind _z_2 (Math|Vector|BreakVector _worldlocation))
  (bind _returnvalue_2 (/ _z_2 _z))
  (bind _returnvalue_3 (* _worlddirection _returnvalue_2))
  (bind _returnvalue_4 (* _returnvalue_3 -1.0))
  (bind _returnvalue_5 (+ _worldlocation _returnvalue_4))
  ;[1 1 1] Follow cursor on tick
  (if (Variables|Default|GetTracking%20Cursor?)
    (Transformation|SetWorldLocation (Variables|Default|GetDefaultSceneRoot) (Math|Vector|MakeVector (.x _returnvalue_5) (.y _returnvalue_5) (.Value (Utilities|Map|Find _ship_z_level (.class _ship_details)))) false false)))

(fn ConstructionScript)

(fn SetEntity
  (params (Entity :type Actor%20Class%20Reference))
  (bind _staticmesh (Variables|Default|GetStaticMesh))
  (bind _asship_master (Utilities|Casting|CastToShip_MasterClass Entity))
  (bind _output_get (Variables|Default|SetEntity _asship_master))
  (Components|StaticMesh|SetStaticMesh (Variables|Default|GetStaticMesh) (.Primary%20Static%20Mesh (Utilities|GetClassDefaults _output_get)))
  (for _array_element (Class|MeshComponent|GetMaterialSlotNames _staticmesh)
    (Rendering|Material|SetMaterialbyName _staticmesh _array_element (Variables|Default|GetDynMatIns))))