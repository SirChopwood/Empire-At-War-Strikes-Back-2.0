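; Hyperspace jump actor, named as a preplaced variant, that starts its jump as soon as play begins.
; On BeginPlay it keeps its X and Y but sets its Z from the Entity class defaults, looking up ShipZLevel by the ship's class.
; It then runs the parent BeginPlay and calls BeginJump; Tick is disabled and construction only calls the parent.
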(event EventBeginPlay
  (bind _defaultsceneroot (Variables|Default|GetDefaultSceneRoot))
  (bind _entity (Variables|Default|GetEntity))
  (bind _returnvalue (Transformation|GetWorldLocation _defaultsceneroot))
  (bind (_ship_details _ship_stats _hardpoints _active_hardpoints _primary_static_mesh _ship_z_level) (Utilities|GetClassDefaults _entity))
  (Transformation|SetWorldLocation _defaultsceneroot (Math|Vector|MakeVector (.x _returnvalue) (.y _returnvalue) (.Value (Utilities|Map|Find _ship_z_level (.class _ship_details)))) false false)
  (|CallParentFunction)
  (CallFunction|BeginJump))

(event EventTick
  (params (DeltaSeconds :type Float%20%28single-precision%29))
  (|CallParentFunction DeltaSeconds) ; This node is disabled and will not be called.\nDrag off pins to build functionality.
)

(fn ConstructionScript
  (|CallParentFunction))